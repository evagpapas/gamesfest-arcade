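; BP_DialogueOption is a floating dialogue answer bubble that writes AnswerText to its text render every tick.
; From BeginPlay, StartMovingBubble re-arms itself on a looping two-second timer, saves the current location and picks a random X/Z point within set bounds.
; The actor snaps to that relative point, then a timeline adds the lerp between saved and new locations as a swept world offset each update, rather than setting position.
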(event `self.ReceiveTick`
  (params (DeltaSeconds :type "Float (single-precision)"))
  (`TextRenderComponent.K2_SetText` (`self.TextRender`) (`KismetTextLibrary.Conv_StringToText` (`self.AnswerText`))))

(event `GetCurrentLocation`
  (set `self.CurrentLocation` (`self.K2_GetActorLocation`)))

(event `StartMovingBubble`
  (bind _returnvalue (`KismetSystemLibrary.K2_SetTimerDelegate` (delegate `StartMovingBubble`) 2.0 true))
  (set `self.BubbleTimer` _returnvalue)
  (`self.GetCurrentLocation`)
  (`self.Find New Location`)
  (bind (_direction _bubblemovement) (`Timeline|T_BubbleTrajectory` :!via `PlayFromStart`)
    (:`Update`
      (`self.LerpLocation` _bubblemovement)
      (`KismetSystemLibrary.Delay` 1.0))))

(event `self.ReceiveBeginPlay`
  (`self.StartMovingBubble`))

(event `Find New Location`
  (bind _output_get (set `self.NewLocation` (`KismetMathLibrary.MakeVector` (`KismetMathLibrary.RandomFloatInRange` (`self.MinX`) (`self.MaxX`)) 0.0 (`KismetMathLibrary.RandomFloatInRange` (`self.MinY`) (`self.MaxY`)))))
  (`self.K2_SetActorRelativeLocation` _output_get)
  (`KismetSystemLibrary.PrintString` "New Location" true true (struct :`G` 0.66 :`B` 1.0 :`A` 1.0) 1.0 "2"))

(event `LerpLocation`
  (params (BubbleMovement :type "Float (double-precision)"))
  (`self.K2_AddActorWorldOffset` (`KismetMathLibrary.VLerp` (`self.CurrentLocation`) (`self.NewLocation`) BubbleMovement) true))

(fn `UserConstructionScript`)