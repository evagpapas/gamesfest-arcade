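; BP_Tamagotchi is a virtual pet whose cat sprite changes appearance as its affection level rises.
; An Evolve event takes the affection level and switches on it to set the matching evolution sprite on the TamagotchiSprite component.
; The highest handled level and any unmatched value share the same sprite, and the Blueprint has no other active logic.
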(event `Evolve`
  (params (AffectionLevel :type Integer))
  (switch `int` AffectionLevel
    (:`Default`
      (`PaperSpriteComponent.SetSprite` (`self.TamagotchiSprite`) "/Game/Core/Assets/All_cat_evolutions_TamagotchiSprite_15.All_cat_evolutions_TamagotchiSprite_15" :!label _label))
    (:`0`
      (`PaperSpriteComponent.SetSprite` (`self.TamagotchiSprite`) "/Game/Core/Assets/All_cat_evolutions_TamagotchiSprite_0.All_cat_evolutions_TamagotchiSprite_0"))
    (:`1`
      (`PaperSpriteComponent.SetSprite` (`self.TamagotchiSprite`) "/Game/Core/Assets/All_cat_evolutions_TamagotchiSprite_3.All_cat_evolutions_TamagotchiSprite_3"))
    (:`2`
      (`PaperSpriteComponent.SetSprite` (`self.TamagotchiSprite`) "/Game/Core/Assets/All_cat_evolutions_TamagotchiSprite_4.All_cat_evolutions_TamagotchiSprite_4"))
    (:`3`
      (`PaperSpriteComponent.SetSprite` (`self.TamagotchiSprite`) "/Game/Core/Assets/All_cat_evolutions_TamagotchiSprite_8.All_cat_evolutions_TamagotchiSprite_8"))
    (:`4`
      (`PaperSpriteComponent.SetSprite` (`self.TamagotchiSprite`) "/Game/Core/Assets/All_cat_evolutions_TamagotchiSprite_11.All_cat_evolutions_TamagotchiSprite_11"))
    (:`5`
      (`PaperSpriteComponent.SetSprite` (`self.TamagotchiSprite`) "/Game/Core/Assets/All_cat_evolutions_TamagotchiSprite_12.All_cat_evolutions_TamagotchiSprite_12"))
    (:`6`
      (goto _label))))

(fn `UserConstructionScript`)