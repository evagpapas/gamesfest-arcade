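; GM_Menu is the main menu game mode that builds the title screen when play begins.
; BeginPlay adds the WB_MainScreen widget to the viewport and spawns a BP_Background actor with the title screen sprite.
; It also adds the IMC_MainMenu Enhanced Input mapping context to the first player controller and tells BP_GameInstance to play music.
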(event `self.ReceiveBeginPlay`
  (bind _returnvalue (`|CreateWidget` "/Game/Core/BPs/Widgets/WB_MainScreen.WB_MainScreen_C" (`GameplayStatics.GetPlayerController` 0)))
  (`UserWidget.AddToViewport` _returnvalue 0)
  (bind _returnvalue_2 (`|SpawnActorFromClass` "/Game/Core/BPs/BP_Background.BP_Background_C" (`KismetMathLibrary.MakeTransform` (0.0 0.0 0.0)) "Undefined" "MultiplyWithRoot" null null))
  (`PaperSpriteComponent.SetSprite` (`/Game/Core/BPs/BP_Background.BackgroundSprite` _returnvalue_2) "/Game/Core/Assets/TitleScreenFINAL_ALT_Sprite.TitleScreenFINAL_ALT_Sprite")
  (`EnhancedInputSubsystemInterface.AddMappingContext` (pcsubsystem `EnhancedInputLocalPlayerSubsystem` (`GameplayStatics.GetPlayerController` 0)) "/Game/Core/IMC_MainMenu.IMC_MainMenu" 0 (struct))
  (bind _asbp_game_instance (cast `/Game/Core/BPs/BP_GameInstance` (`GameplayStatics.GetGameInstance`)))
  (`/Game/Core/BPs/BP_GameInstance.PlayMusic` _asbp_game_instance))

(fn `UserConstructionScript`)