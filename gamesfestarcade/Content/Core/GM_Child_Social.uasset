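; Game mode for the Social minigame, a dialogue quiz where the picked answer raises or lowers affection.
; On BeginPlay it spawns three dialogue option actors, hides the radial timer, and fills them with shuffled answers from a random data table question.
; A click traces from the mouse to an option, compares it to the correct answer, updates affection and needs through the game instance, then returns to MainLevel.
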(event `ClickEvent`
  (bind (_worldlocation _worlddirection) (`PlayerController.DeprojectMousePositionToWorld` (`GameplayStatics.GetPlayerController` 0)))
  (bind _outhit (`KismetSystemLibrary.LineTraceSingle` _worldlocation (+ _worldlocation (* _worlddirection 1000.0)) "TraceTypeQuery2"))
  (bind _output_get (set `self.Out Hit Hit Actor` (`.HitActor` (`GameplayStatics.BreakHitResult` _outhit))))
  (if (== (`GameplayStatics.GetObjectClass` _output_get) "/Game/Core/BPs/BP_DialogueOption.BP_DialogueOption_C")
    (bind _asbp_dialogue_option (cast `/Game/Core/BPs/BP_DialogueOption` (`self.Out Hit Hit Actor`)))
    (if (== (`self.CorrectAnswer`) (`/Game/Core/BPs/BP_DialogueOption.AnswerText` _asbp_dialogue_option))
      (`/Game/Core/BPs/BP_GameInstance.IncreaseAffection` (`self.As BP Game Instance`))
      (else
        (`/Game/Core/BPs/BP_GameInstance.DecreaseAffection` (`self.As BP Game Instance`))))
    (`/Game/Core/BPs/BP_GameInstance.UpdateNeeds` (`self.As BP Game Instance`))
    (`GameplayStatics.OpenLevel` "MainLevel")))

(event `self.ReceiveBeginPlay`
  (`parent.ReceiveBeginPlay`)
  (`self.ChangeBackground` "/Game/Core/Assets/BGs/Talking_Sprite.Talking_Sprite")
  (`self.SetGameName` "Social")
  (`Widget.SetVisibility` (`/Game/Core/BPs/Widgets/WB_Minigame.WB_RadialTimer` (`self.WB_Minigame`)) "Hidden")
  (bind _returnvalue (`|SpawnActorFromClass` "/Game/Core/BPs/BP_DialogueOption.BP_DialogueOption_C" (`KismetMathLibrary.MakeTransform` (-600.0 0.5 0.0)) "Undefined" "MultiplyWithRoot" null null))
  (set `self.BP_Option1` _returnvalue)
  (bind _returnvalue_2 (`|SpawnActorFromClass` "/Game/Core/BPs/BP_DialogueOption.BP_DialogueOption_C" (`KismetMathLibrary.MakeTransform` (0.0 1.0 0.0)) "Undefined" "MultiplyWithRoot" null null))
  (set `self.BP_Option2` _returnvalue_2)
  (bind _returnvalue_3 (`|SpawnActorFromClass` "/Game/Core/BPs/BP_DialogueOption.BP_DialogueOption_C" (`KismetMathLibrary.MakeTransform` (600.0 2.0 0.0)) "Undefined" "MultiplyWithRoot" null null))
  (set `self.BP_Option3` _returnvalue_3)
  (`self.GetRandomQuestion`)
  (`self.AssignChoices`)
  (`self.PassToDialogueBubbles`)
  (set `self.MappingContext` "/Game/Core/IMC_Talk.IMC_Talk")
  (`self.SetMapping`)
  (bind _returnvalue_4 (`|CreateWidget` "/Game/Core/BPs/Widgets/WB_QuestionOverlay.WB_QuestionOverlay_C" (`GameplayStatics.GetPlayerController` 0)))
  (`UserWidget.AddToViewport` _returnvalue_4 0))

(event `GetRandomQuestion`
  (bind _outrownames (`DataTableFunctionLibrary.GetDataTableRowNames` (`self.DataTable`)))
  (bind _returnvalue (`|GetDataTableRow` (`self.DataTable`) (`|GetArrayItem` _outrownames (`KismetMathLibrary.RandomIntegerInRange` 0 (- (`KismetArrayLibrary.Array_Length` _outrownames) 1))))
    (:`then`
      (bind _output_get (set `self.CurrentStruct` _returnvalue))
      (bind (_question _correctanswer _incorrectanswer) (break `/Game/Core/BPs/Struct_Talk` _output_get))
      (set `self.CurrentQuestion` _question)
      (bind _output_get_2 (set `self.CorrectAnswer` _correctanswer))
      (bind _output_get_3 (set `self.AnswerChoices` _incorrectanswer))
      (`KismetArrayLibrary.Array_Add` _output_get_3 _output_get_2)
      (`KismetArrayLibrary.Array_Shuffle` (`self.AnswerChoices`)))))

(event `AssignChoices`
  (for (_array_element _array_index) (`self.AnswerChoices`)
    (set `self.TempAnswer` _array_element)
    (bind _output_get (set `self.Array Index` _array_index))
    (switch `int` _output_get
      (:`0`
        (set `self.ChoiceA` (`self.TempAnswer`)))
      (:`1`
        (set `self.ChoiceB` (`self.TempAnswer`)))
      (:`2`
        (set `self.ChoiceC` (`self.TempAnswer`))))))

(event `PassToDialogueBubbles`
  (set `/Game/Core/BPs/BP_DialogueOption.AnswerText` (`self.ChoiceA`) (`self.BP_Option1`))
  (set `/Game/Core/BPs/BP_DialogueOption.AnswerText` (`self.ChoiceB`) (`self.BP_Option2`))
  (set `/Game/Core/BPs/BP_DialogueOption.AnswerText` (`self.ChoiceC`) (`self.BP_Option3`)))

(event `ApplyQuestion`
  (bind _returnvalue (`GameplayStatics.GetActorOfClass` "/Game/Core/BPs/BP_QuestionText.BP_QuestionText_C"))
  (`TextRenderComponent.K2_SetText` (`/Game/Core/BPs/BP_QuestionText.TextRender` _returnvalue) (`KismetTextLibrary.Conv_StringToText` (`self.CurrentQuestion`))))

(fn `UserConstructionScript`
  (`parent.UserConstructionScript`))