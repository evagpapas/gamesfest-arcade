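; Tamagotchi game mode that tracks and drains four pet needs: Social, Hunger, Fun and Clean.
; Every Tick, DepleteNeeds subtracts a separate random amount, scaled by DepletionMultiplier, from each bar and clamps it between 0 and 100.
; Depletion is per frame, with no Delta Seconds scaling.
; Tick then prints all four values as keyed debug strings.
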(event `self.ReceiveTick`
  (params (DeltaSeconds :type "Float (single-precision)"))
  (`self.DepleteNeeds`)
  (`KismetSystemLibrary.PrintString` (`KismetStringLibrary.Conv_DoubleToString` (`self.SocialBar`)) true true (struct :`G` 0.66 :`B` 1.0 :`A` 1.0) 2.0 "1")
  (`KismetSystemLibrary.PrintString` (`KismetStringLibrary.Conv_DoubleToString` (`self.HungerBar`)) true true (struct :`G` 0.66 :`B` 1.0 :`A` 1.0) 2.0 "2")
  (`KismetSystemLibrary.PrintString` (`KismetStringLibrary.Conv_DoubleToString` (`self.FunBar`)) true true (struct :`G` 0.66 :`B` 1.0 :`A` 1.0) 2.0 "3")
  (`KismetSystemLibrary.PrintString` (`KismetStringLibrary.Conv_DoubleToString` (`self.CleanBar`)) true true (struct :`G` 0.66 :`B` 1.0 :`A` 1.0) 2.0 "4"))

(event `DepleteNeeds`
  (bind _depletionvalue (`self.RandomDepletionValue`))
  (set `self.SocialBar` (`KismetMathLibrary.FClamp` (- (`self.SocialBar`) _depletionvalue) 0.0 100.0))
  (bind _depletionvalue_2 (`self.RandomDepletionValue`))
  (set `self.HungerBar` (`KismetMathLibrary.FClamp` (- (`self.HungerBar`) _depletionvalue_2) 0.0 100.0))
  (bind _depletionvalue_3 (`self.RandomDepletionValue`))
  (set `self.FunBar` (`KismetMathLibrary.FClamp` (- (`self.FunBar`) _depletionvalue_3) 0.0 100.0))
  (bind _depletionvalue_4 (`self.RandomDepletionValue`))
  (set `self.CleanBar` (`KismetMathLibrary.FClamp` (- (`self.CleanBar`) _depletionvalue_4) 0.0 100.0)))

(fn `RandomDepletionValue`
  (returns (DepletionValue :type "Float (double-precision)"))
  (bind _output_get (set `self.TempDepletion` (* (`KismetMathLibrary.RandomFloatInRange` 1.0 5.0) (`self.DepletionMultiplier`))))
  (return _output_get))

(fn `UserConstructionScript`)