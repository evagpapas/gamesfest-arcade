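; Player controller for a Tamagotchi-style pet game that shows the mouse cursor and routes input to level actors.
; Two left-click input actions look up the Social and Clean GM_Child actors by class and call their ClickEvent.
; Any-key input removes the main menu mapping context and opens MainLevel.
; The 0 key, apparently a debug shortcut, increments BP_Tamagotchi's AffectionLevel and calls Evolve.
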(event `self.ReceiveBeginPlay`
  (set `PlayerController.bShowMouseCursor` true (`GameplayStatics.GetPlayerController` 0)))

(event `EnhancedInput|/Game/Core/IA_T_LMB`
  (params (ActionValue :type Boolean) (ElapsedSeconds :type "Float (double-precision)") (TriggeredSeconds :type "Float (double-precision)") (InputAction :type "InputAction Object Reference" :default "/Game/Core/IA_T_LMB.IA_T_LMB"))
  (:`Started`
    (bind _returnvalue (`GameplayStatics.GetActorOfClass` "/Game/Core/GM_Child_Social.GM_Child_Social_C"))
    (`/Game/Core/GM_Child_Social.ClickEvent` _returnvalue)))

(event `EnhancedInput|/Game/Core/IA_C_LMB`
  (params (ActionValue :type Boolean) (ElapsedSeconds :type "Float (double-precision)") (TriggeredSeconds :type "Float (double-precision)") (InputAction :type "InputAction Object Reference" :default "/Game/Core/IA_C_LMB.IA_C_LMB"))
  (:`Started`
    (bind _returnvalue (`GameplayStatics.GetActorOfClass` "/Game/Core/GM_Child_Clean.GM_Child_Clean_C"))
    (`/Game/Core/GM_Child_Clean.ClickEvent` _returnvalue)))

(event `Key|Zero`
  (params (Key :type "Key Structure"))
  (:`Pressed`
    (bind _returnvalue (`GameplayStatics.GetActorOfClass` "/Game/Core/BPs/BP_Tamagotchi.BP_Tamagotchi_C"))
    (bind _result (`/Engine/EditorBlueprintResources/StandardMacros.IncrementInt` (`/Game/Core/BPs/BP_Tamagotchi.AffectionLevel` _returnvalue))
      (:`  `
        (`/Game/Core/BPs/BP_Tamagotchi.Evolve` _returnvalue _result)))))

(event `EnhancedInput|/Game/Core/IA_AnyKey`
  (params (ActionValue :type Boolean) (ElapsedSeconds :type "Float (double-precision)") (TriggeredSeconds :type "Float (double-precision)") (InputAction :type "InputAction Object Reference" :default "/Game/Core/IA_AnyKey.IA_AnyKey"))
  (:`Started`
    (`EnhancedInputSubsystemInterface.RemoveMappingContext` (pcsubsystem `EnhancedInputLocalPlayerSubsystem` (`GameplayStatics.GetPlayerController` 0)) "/Game/Core/IMC_MainMenu.IMC_MainMenu" (struct))
    (`GameplayStatics.OpenLevel` "MainLevel")))

(fn `UserConstructionScript`)