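; Base game mode for minigames, providing shared setup, countdown and win/lose flow, with level setup meant to be altered in child game modes.
; On BeginPlay it spawns a swappable sprite background, creates the minigame widget and caches controller and game instance references.
; Helpers toggle an Enhanced Input mapping context, set the activity label and hide the radial timer.
; A one-second timer counts down to a win; winning or losing adjusts affection, plays a sound and returns to MainLevel.
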(event `RemoveMapping`
  ;[1 0.2745 0.8902] Remove mapping context
  (`EnhancedInputSubsystemInterface.RemoveMappingContext` (pcsubsystem `EnhancedInputLocalPlayerSubsystem` (`self.Bp_PlayerController`)) (`self.MappingContext`) (struct)))

(event `SetMapping`
  ;[1 0.2745 0.8902] Set Mapping Context
  (`EnhancedInputSubsystemInterface.AddMappingContext` (pcsubsystem `EnhancedInputLocalPlayerSubsystem` (`self.Bp_PlayerController`)) (`self.MappingContext`) 0 (struct)))

(event `self.ReceiveBeginPlay`
  ;[1 0.2745 0.8902] Begin Play
  (`self.LevelSetUp`)
  (bind _asbp_player_controller (cast `/Game/Core/BP_PlayerController` (`GameplayStatics.GetPlayerController` 0)))
  (set `self.Bp_PlayerController` _asbp_player_controller)
  (bind _asbp_game_instance (cast `/Game/Core/BPs/BP_GameInstance` (`GameplayStatics.GetGameInstance`)))
  (set `self.BP_GI` _asbp_game_instance)
  (bind _asgm_tamagotchi (cast `/Game/Core/GM_Tamagotchi` (`GameplayStatics.GetGameMode`)))
  (set `self.GM_Tamagotchi` _asgm_tamagotchi)
  (`KismetSystemLibrary.Delay` 1.0))

(event `LevelSetUp`
  ;[1 0.2745 0.8902] Level Set Up (alter variables in child game modes)
  (bind _returnvalue (`|SpawnActorFromClass` "/Game/Core/BPs/BP_Background.BP_Background_C" (`KismetMathLibrary.MakeTransform` (0.0 0.0 0.0)) "Undefined" "MultiplyWithRoot" null null))
  (set `self.BP_Background` _returnvalue)
  (bind _returnvalue_2 (`|CreateWidget` "/Game/Core/BPs/Widgets/WB_Minigame.WB_Minigame_C" (`GameplayStatics.GetPlayerController` 0)))
  (bind _output_get (set `self.WB_Minigame` _returnvalue_2))
  (`UserWidget.AddToViewport` _output_get 0))

(event `SetActivityType`
  (params (GameName :type String))
  (bind _returnvalue (`KismetTextLibrary.Conv_StringToText` GameName))
  ;[1 0.2745 0.8902] ActivityType String
  (set `self.ActivityType` _returnvalue)
  (set `/Game/Core/BPs/Widgets/WB_Minigame.ActivityType` _returnvalue (`self.WB_Minigame`)))

(event `UpdateTimer`
  ;[1 0.2745 0.8902] Update Timer
  (bind _returnvalue (`KismetSystemLibrary.K2_SetTimerDelegate` (delegate `UpdateTimer`) 1.0 true))
  (set `self.Timer_Minigame` _returnvalue)
  (if (> (`self.TimeLeft`) 0.0)
    (set `self.TimeLeft` (- (`self.TimeLeft`) 1.0))
    (else
      (`self.TimeOut`))))

(event `ChangeBackground`
  (params (BackgroundSprite :type "PaperSprite Object Reference"))
  ;[1 0.2745 0.8902] Change background texture
  (`PaperSpriteComponent.SetSprite` (`/Game/Core/BPs/BP_Background.BackgroundSprite` (`self.BP_Background`)) BackgroundSprite))

(event `StopTimer`
  ;[1 0.2745 0.8902] StopTimer
  (`KismetSystemLibrary.K2_ClearAndInvalidateTimerHandle` (`self.Timer_Minigame`)))

(event `Win`
  ;[1 0.2745 0.8902] Win
  (`self.RemoveMapping`)
  (`/Game/Core/BPs/BP_GameInstance.PlusAffection` (`self.BP_GI`))
  (`GameplayStatics.OpenLevel` "MainLevel")
  (`GameplayStatics.PlaySound2D` "/Game/Core/Assets/SFX/meterincrease.meterincrease" 1.0 1.0 0.0 null null))

(event `TimeOut`
  ;[1 0.2745 0.8902] No time left on timer
  (`self.StopTimer`)
  (set `self.TimeLeft` (`self.MaxTime`))
  (`self.Win`)
  (`GameplayStatics.OpenLevel` "MainLevel"))

(event `Lose`
  ;[1 0.2745 0.8902] Lose
  (`self.RemoveMapping`)
  (`/Game/Core/BPs/BP_GameInstance.MinusAffection` (`self.BP_GI`))
  (`GameplayStatics.OpenLevel` "MainLevel")
  (`GameplayStatics.PlaySound2D` "/Game/Core/Assets/SFX/fail.fail" 1.0 1.0 0.0 null null))

(event `HideTimer`
  ;[1 0.2745 0.8902] Hide Timer Widget
  (`Widget.SetVisibility` (`/Game/Core/BPs/Widgets/WB_Minigame.WB_RadialTimer` (`self.WB_Minigame`)) "Hidden"))

(fn `UserConstructionScript`)